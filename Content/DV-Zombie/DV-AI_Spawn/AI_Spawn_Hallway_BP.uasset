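; Hallway zombie spawner that fills its Box volume with behavior-tree-driven zombies once SpawnAIAtHallway enables it.
; While enabled, Tick checks that fewer than 50 Spawned_Zombie_BP actors exist in the world.
; Under that cap, a DoOnce spawns an initial burst of six at random points in the box.
; A Delay on Tick then adds one more roughly every two seconds, with debug prints.
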(event Custom|Spawn%20AI%20At%20Hallway
  (Variables|Default|SetAI%20Spawn%20Allowed? true)
  (Development|PrintString "Hallway AI Are Spawning" true true "(R=1.000000,G=0.000000,B=0.916799,A=1.000000)"))

(event EventBeginPlay)

(event EventTick
  (params (DeltaSeconds :type Float%20%28single-precision%29))
  (bind _box (Variables|Default|GetBox))
  (bind _box_2 (Variables|Default|GetBox))
  (bind _box_3 (Variables|Default|GetBox))
  (bind _box_4 (Variables|Default|GetBox))
  (bind _box_5 (Variables|Default|GetBox))
  (bind _box_6 (Variables|Default|GetBox))
  (bind _box_7 (Variables|Default|GetBox))
  (if (Variables|Default|GetAI%20Spawn%20Allowed?)
    (bind _outactors (Actor|GetAllActorsOfClass "/Game/DV-Zombie/DV-Spawned_Zombie_AI/Spawned_Zombie_BP.Spawned_Zombie_BP_C"))
    (if (< (Utilities|Array|Length _outactors) 50)
      (Utilities|FlowControl|Sequence
        (:then_0
          (Utilities|FlowControl|DoOnce false
            (:Completed
              (AI|SpawnAIFromClass "/Game/DV-Zombie/DV-Spawned_Zombie_AI/Spawned_Zombie_BP.Spawned_Zombie_BP_C" "/Game/DV-Zombie/DV-Spawned_Zombie_AI/Spawned_Zombie_BehaviorTree.Spawned_Zombie_BehaviorTree" (Math|Random|RandomPointinBoundingBox (Transformation|GetWorldLocation _box_7) (Components|Box|GetScaledBoxExtent _box_7)) "0, 0, 0" false 0)
              (AI|SpawnAIFromClass "/Game/DV-Zombie/DV-Spawned_Zombie_AI/Spawned_Zombie_BP.Spawned_Zombie_BP_C" "/Game/DV-Zombie/DV-Spawned_Zombie_AI/Spawned_Zombie_BehaviorTree.Spawned_Zombie_BehaviorTree" (Math|Random|RandomPointinBoundingBox (Transformation|GetWorldLocation _box_3) (Components|Box|GetScaledBoxExtent _box_3)) "0, 0, 0" false 0)
              (AI|SpawnAIFromClass "/Game/DV-Zombie/DV-Spawned_Zombie_AI/Spawned_Zombie_BP.Spawned_Zombie_BP_C" "/Game/DV-Zombie/DV-Spawned_Zombie_AI/Spawned_Zombie_BehaviorTree.Spawned_Zombie_BehaviorTree" (Math|Random|RandomPointinBoundingBox (Transformation|GetWorldLocation _box_4) (Components|Box|GetScaledBoxExtent _box_4)) "0, 0, 0" false 0)
              (AI|SpawnAIFromClass "/Game/DV-Zombie/DV-Spawned_Zombie_AI/Spawned_Zombie_BP.Spawned_Zombie_BP_C" "/Game/DV-Zombie/DV-Spawned_Zombie_AI/Spawned_Zombie_BehaviorTree.Spawned_Zombie_BehaviorTree" (Math|Random|RandomPointinBoundingBox (Transformation|GetWorldLocation _box_5) (Components|Box|GetScaledBoxExtent _box_5)) "0, 0, 0" false 0)
              (AI|SpawnAIFromClass "/Game/DV-Zombie/DV-Spawned_Zombie_AI/Spawned_Zombie_BP.Spawned_Zombie_BP_C" "/Game/DV-Zombie/DV-Spawned_Zombie_AI/Spawned_Zombie_BehaviorTree.Spawned_Zombie_BehaviorTree" (Math|Random|RandomPointinBoundingBox (Transformation|GetWorldLocation _box_6) (Components|Box|GetScaledBoxExtent _box_6)) "0, 0, 0" false 0)
              (AI|SpawnAIFromClass "/Game/DV-Zombie/DV-Spawned_Zombie_AI/Spawned_Zombie_BP.Spawned_Zombie_BP_C" "/Game/DV-Zombie/DV-Spawned_Zombie_AI/Spawned_Zombie_BehaviorTree.Spawned_Zombie_BehaviorTree" (Math|Random|RandomPointinBoundingBox (Transformation|GetWorldLocation _box) (Components|Box|GetScaledBoxExtent _box)) "0, 0, 0" false 0)
              (Development|PrintString "Spawned 6 Zombies" true true "(R=1.000000,G=0.837795,B=0.000000,A=1.000000)"))))
        (:then_1
          (Utilities|FlowControl|Delay 2.0)
          (AI|SpawnAIFromClass "/Game/DV-Zombie/DV-Spawned_Zombie_AI/Spawned_Zombie_BP.Spawned_Zombie_BP_C" "/Game/DV-Zombie/DV-Spawned_Zombie_AI/Spawned_Zombie_BehaviorTree.Spawned_Zombie_BehaviorTree" (Math|Random|RandomPointinBoundingBox (Transformation|GetWorldLocation _box_2) (Components|Box|GetScaledBoxExtent _box_2)) "0, 0, 0" false 0)
          (Development|PrintString "Spawned Zombie At Hallway" true true "(R=1.000000,G=0.000000,B=0.000000,A=1.000000)"))))))

(fn ConstructionScript)