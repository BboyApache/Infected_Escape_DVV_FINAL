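; Zombie spawner actor for the Big Room that stays idle until its SpawnAIInBigRoom event enables spawning.
; Once enabled, Tick counts all Spawned_Zombie_BP actors and, while fewer than 50 exist, uses a Delay to pace spawns about one second apart.
; Each zombie spawns with its behavior tree at a random point inside the Box component, with debug prints on activation and spawn.
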(event Custom|Spawn%20AI%20In%20Big%20Room
  (Variables|Default|SetAI%20Spawn%20Allowed? true)
  (Development|PrintString "Big Room AI Are Spawning" true true "(R=1.000000,G=0.000000,B=0.838576,A=1.000000)"))

(event EventBeginPlay)

(event EventTick
  (params (DeltaSeconds :type Float%20%28single-precision%29))
  (bind _box (Variables|Default|GetBox))
  (if (Variables|Default|GetAI%20Spawn%20Allowed?)
    (bind _outactors (Actor|GetAllActorsOfClass "/Game/DV-Zombie/DV-Spawned_Zombie_AI/Spawned_Zombie_BP.Spawned_Zombie_BP_C"))
    (if (< (Utilities|Array|Length _outactors) 50)
      (Utilities|FlowControl|Delay 1.0)
      (AI|SpawnAIFromClass "/Game/DV-Zombie/DV-Spawned_Zombie_AI/Spawned_Zombie_BP.Spawned_Zombie_BP_C" "/Game/DV-Zombie/DV-Spawned_Zombie_AI/Spawned_Zombie_BehaviorTree.Spawned_Zombie_BehaviorTree" (Math|Random|RandomPointinBoundingBox (Transformation|GetWorldLocation _box) (Components|Box|GetScaledBoxExtent _box)) "0, 0, 0" false 0)
      (Development|PrintString "Spawned Zombie In Big Room" true true "(R=1.000000,G=0.000000,B=0.838576,A=1.000000)"))))

(fn ConstructionScript)