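; Zombie enemy character that loses health to first-person projectile hits and attacks the player.
; An overlap component plays grunts when the player enters it, and the attack event waits, plays a montage and sphere-traces ahead to damage the player.
; Tick triggers a one-time death when health drops below zero: sound, controller detach, disabled movement, then a delayed ragdoll and destroy.
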(event OnComponentBeginOverlap(PlaySound)
  (params (OverlappedComponent :type Primitive%20Component%20Object%20Reference) (OtherActor :type Actor%20Object%20Reference) (OtherComp :type Primitive%20Component%20Object%20Reference) (OtherBodyIndex :type Integer) (bFromSweep :type Boolean) (SweepResult :type Hit%20Result%20Structure%20%28by%20ref%29))
  ;[1 1 1] Play Grunt/Chase Sound when near player
  (if (== OtherActor (Variables|Default|GetFirst%20Person%20Character%20Reference))
    (Audio|PlaySoundatLocation "/Game/DV-Zombie/DV-Zombie_Sounds/Grunts_Cue.Grunts_Cue" (Transformation|GetWorldLocation (Variables|Collision|GetCapsuleComponent)) "0, 0, 0" 1.0 1.0 0.0 "/Game/DV-Zombie/DV-Zombie_Sounds/Zombie_Death_Sound_Attenuation.Zombie_Death_Sound_Attenuation" 0 0)))

(event Custom|Death
  ;[1 1 1] Death Event
  (Utilities|FlowControl|DoOnce false
    (:Completed
      (Audio|PlaySoundatLocation "/Game/DV-Zombie/DV-Zombie_Sounds/MonsterDeathFinal_Cue.MonsterDeathFinal_Cue" (Transformation|GetWorldLocation (Variables|Collision|GetCapsuleComponent)) "0, 0, 0" 1.0 1.0 0.0 "/Game/DV-Zombie/DV-Zombie_Sounds/Zombie_Death_Sound_Attenuation.Zombie_Death_Sound_Attenuation" 0 0)
      (Collision|SetCollisionEnabled (Variables|Collision|GetCapsuleComponent) "NoCollision")
      (Pawn|Components|CharacterMovement|DisableMovement (Variables|Character|GetCharacterMovement))
      (Class|Pawn|DetachfromControllerPendingDestroy)
      (Utilities|FlowControl|Delay 1.4)
      (Collision|SetCollisionEnabled (Variables|Character|GetMesh) "QueryAndPhysics")
      (Physics|SetSimulatePhysics (Variables|Character|GetMesh) true)
      (Utilities|FlowControl|Delay 5.0)
      (Actor|DestroyActor))))

(event Custom|Positioned%20Zombie%20Attack
  (bind _returnvalue (Transformation|GetActorLocation))
  ;[1 1 1] Attack
  (Utilities|FlowControl|Delay 2.0)
  (Animation|Montage|PlayMontage (Variables|Character|GetMesh) "/Game/DV-Zombie/DV-Zombie_Animation/Animation_Montages/Hip_Up_Animation/zombie_attack_Montage.zombie_attack_Montage"
    (:then
      (bind _outhit (Collision|SphereTraceByChannel _returnvalue (+ _returnvalue (* (Transformation|GetActorUpVector) 4e+01) (* (Transformation|GetActorForwardVector) 1.4e+02)) 8e+01 "TraceTypeQuery3" false (Actor|GetAllChildActors true) "None"))
      (if (.bSuccess (Utilities|Casting|CastToFirstPersonCharacterClass (Utilities|GetClass (.HitActor (Collision|BreakHitResult _outhit)))))
        (Default|TakeDamage (Variables|Default|GetFirst%20Person%20Character%20Reference))))))

(event EventBeginPlay
  ;[1 1 1] On Begin Play; Set Health and Fisrt Person Character Reference
  (Variables|Default|SetHealth 1e+02)
  (bind _asfirst_person_character (Utilities|Casting|CastToFirstPersonCharacter (Game|Player|GetPlayerPawn 0)))
  (Variables|Default|SetFirst%20Person%20Character%20Reference _asfirst_person_character))

(event EventTick
  (params (DeltaSeconds :type Float%20%28single-precision%29))
  ;[1 1 1] Event Tick Debug Display Health and Checks Health Condition
  (if (< (Variables|Default|GetHealth) 0.0)
    (CallFunction|Death)))

(event Collision|EventHit
  (params (MyComp :type Primitive%20Component%20Object%20Reference) (Other :type Actor%20Object%20Reference) (OtherComp :type Primitive%20Component%20Object%20Reference) (bSelfMoved :type Boolean) (HitLocation :type Vector :default "0, 0, 0") (HitNormal :type Vector :default "0, 0, 0") (NormalImpulse :type Vector :default "0, 0, 0") (Hit :type Hit%20Result%20Structure%20%28by%20ref%29))
  ;[1 1 1] When Projectile Hits; -10 Health
  (if (.bSuccess (Utilities|Casting|CastToFirstPersonProjectileClass (Utilities|GetClass Other)))
    (Variables|Default|SetHealth (- (Variables|Default|GetHealth) 13.0))))

(fn ConstructionScript)